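; Game instance that handles showing the main menu and switching levels.
; Menu events create the main menu widget, store it on BP_MainGameMode and add it to or remove it from the viewport.
; Level loading looks up the target in LevelsArray, opens it by object reference, then calls CallOnInit on the game mode after a short delay.
; UnloadTargetLevel is an empty stub.
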(event EventLoadMainMenu
  (bind _asbp_main_game_mode (Utilities|Casting|CastToBP_MainGameMode (Game|GetGameMode)))
  (Variables|/Game/Blueprints/Gameplay/BP_MainGameMode.BP_MainGameMode_C|GetMainMenuWidget _asbp_main_game_mode
    (:then)
    (:else
      (bind _returnvalue (UserInterface|CreateWidget "/Game/UI/WBP_MainMenu.WBP_MainMenu_C" (Game|GetPlayerController 0)))
      (bind _output_get (Variables|/Game/Blueprints/Gameplay/BP_MainGameMode.BP_MainGameMode_C|SetMainMenuWidget _asbp_main_game_mode _returnvalue))
      (UserInterface|Viewport|AddtoViewport _output_get 0))))

(event EventLoadTargetLevel
  (params (TargetLevel :type String))
  (bind _levelsarray (Variables|Default|GetLevelsArray))
  (bind (_value _returnvalue) (Utilities|Map|Find _levelsarray TargetLevel))
  (if _returnvalue
    (Game|OpenLevel(byObjectReference) _value)
    (Utilities|FlowControl|Delay 0.2)
    (bind _asbp_main_game_mode (Utilities|Casting|CastToBP_MainGameMode (Game|GetGameMode)))
    (Default|CallOnInit _asbp_main_game_mode)))

(event EventUnloadMainMenu
  (bind _mainmenuwidget (Variables|/Game/Blueprints/Gameplay/BP_MainGameMode.BP_MainGameMode_C|GetMainMenuWidget (stale EventLoadMainMenu _asbp_main_game_mode))
    (:then
      (Widget|RemovefromParent _mainmenuwidget))
    (:else)))

(event EventUnloadTargetLevel
  (params (TargetLevel :type String)))