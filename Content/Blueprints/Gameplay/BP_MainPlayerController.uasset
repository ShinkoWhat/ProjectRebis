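; Main player controller that drives the light-attack combo, pause screen and color-vision-deficiency hotkeys.
; Light attack plays the current weapon's combo montage or, through a gate opened and closed by combo events, chains its next section; releasing resets the Pegasus sword's attack count.
; Tick scales the active montage's play rate from 1x to 2x with the game mode's multiplier.
; Escape pauses the game and stopwatch and shows the pause widget.
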(event Custom|NextComboStep
  (Utilities|FlowControl|Gate false
    (:Exit
      (Class|AnimInstance|MontageSetNextSection (Components|SkeletalMesh|GetAnimInstance (Variables|/Script/Engine.Character|GetMesh (stale Input|EnhancedActionEvents|EnhancedInputActionIA_LightAttack _asbp_main_player))) (Animation|Montage|MontageGetCurrentSection (Components|SkeletalMesh|GetAnimInstance (Variables|/Script/Engine.Character|GetMesh (stale Input|EnhancedActionEvents|EnhancedInputActionIA_LightAttack _asbp_main_player))) (Animation|Montage|GetCurrentActiveMontage (Components|SkeletalMesh|GetAnimInstance (Variables|/Script/Engine.Character|GetMesh (stale Input|EnhancedActionEvents|EnhancedInputActionIA_LightAttack _asbp_main_player))))) (Variables|Default|GetNextStep) (Animation|Montage|GetCurrentActiveMontage (Components|SkeletalMesh|GetAnimInstance (Variables|/Script/Engine.Character|GetMesh (stale Input|EnhancedActionEvents|EnhancedInputActionIA_LightAttack _asbp_main_player))))))))

(event Custom|RefreshCombo
  (Utilities|FlowControl|Gate false) ; enters at Open
)

(event Custom|BlockCombo
  (Utilities|FlowControl|Gate false) ; enters at Close
)

(event Custom|OnNextComboStep
  (params (NextStep :type Name))
  (Variables|Default|SetNextStep NextStep)
  (CallFunction|RefreshCombo))

(event Custom|OnClearCombo
  (Variables|Default|SetNextStep "None")
  (CallFunction|BlockCombo))

(event Input|EnhancedActionEvents|EnhancedInputActionIA_LightAttack
  (params (ActionValue :type Boolean) (ElapsedSeconds :type Float%20%28double-precision%29) (TriggeredSeconds :type Float%20%28double-precision%29) (InputAction :type Input%20Action%20Object%20Reference :default "/Game/Input/Actions/IA_LightAttack.IA_LightAttack"))
  (:Triggered
    (bind _asbp_main_player (Utilities|Casting|CastToBP_MainPlayer (Game|GetPlayerCharacter 0)))
    (Utilities|FlowControl|Sequence
      (:then_0
        (if (and (== (Animation|Montage|MontageGetCurrentSection (Components|SkeletalMesh|GetAnimInstance (Variables|/Script/Engine.Character|GetMesh _asbp_main_player)) (Animation|Montage|GetCurrentActiveMontage (Components|SkeletalMesh|GetAnimInstance (Variables|/Script/Engine.Character|GetMesh _asbp_main_player)))) (Animation|Montage|MontageGetCurrentSection (Components|SkeletalMesh|GetAnimInstance (Variables|/Script/Engine.Character|GetMesh _asbp_main_player)) (Variables|/Script/ProjectRebis.BaseWeapon|GetComboMontage (Variables|/Script/ProjectRebis.CharacterBase|GetCurrentWeapon _asbp_main_player)))) (!= (Animation|Montage|MontageGetCurrentSection (Components|SkeletalMesh|GetAnimInstance (Variables|/Script/Engine.Character|GetMesh _asbp_main_player)) (Animation|Montage|GetCurrentActiveMontage (Components|SkeletalMesh|GetAnimInstance (Variables|/Script/Engine.Character|GetMesh _asbp_main_player)))) ""))
          (CallFunction|NextComboStep)
          (else
            (Animation|PlayAnimMontage _asbp_main_player (Variables|/Script/ProjectRebis.BaseWeapon|GetComboMontage (Variables|/Script/ProjectRebis.CharacterBase|GetCurrentWeapon _asbp_main_player)) 1.0 "None"))))
      (:then_1
        (Development|PrintString (Utilities|String|Append (Utilities|String|ToString(Name) (Animation|Montage|MontageGetCurrentSection (Components|SkeletalMesh|GetAnimInstance (Variables|/Script/Engine.Character|GetMesh _asbp_main_player)) (Animation|Montage|GetCurrentActiveMontage (Components|SkeletalMesh|GetAnimInstance (Variables|/Script/Engine.Character|GetMesh _asbp_main_player))))) " / " (Utilities|String|ToString(Name) (Animation|Montage|MontageGetCurrentSection (Components|SkeletalMesh|GetAnimInstance (Variables|/Script/Engine.Character|GetMesh _asbp_main_player)) (Variables|/Script/ProjectRebis.BaseWeapon|GetComboMontage (Variables|/Script/ProjectRebis.CharacterBase|GetCurrentWeapon _asbp_main_player)))))))))
  (:Canceled
    (Variables|Default|GetPlayerCharacterReference :!label _label
      (:then
        (bind _asbp_pegasus_sword (Utilities|Casting|CastToBP_PegasusSword (Variables|/Script/ProjectRebis.CharacterBase|GetCurrentWeapon _asbp_main_player)))
        (Default|CallResetAtkCount _asbp_pegasus_sword))
      (:else)))
  (:Completed
    (goto _label)))

(event EventBeginPlay)

(event EventTick
  (params (DeltaSeconds :type Float%20%28single-precision%29))
  (bind _asbp_main_game_mode (Utilities|Casting|CastToBP_MainGameMode (Game|GetGameMode)))
  (bind _asbp_main_player (Utilities|Casting|CastToBP_MainPlayer (Game|GetPlayerCharacter 0)))
  (Animation|Montage|MontageSetPlayRate (Components|SkeletalMesh|GetAnimInstance (Variables|/Script/Engine.Character|GetMesh _asbp_main_player)) (Animation|Montage|GetCurrentActiveMontage (Components|SkeletalMesh|GetAnimInstance (Variables|/Script/Engine.Character|GetMesh _asbp_main_player))) (Math|Float|Lerp 1.0 2.0 (/ (Variables|/Game/Blueprints/Gameplay/BP_MainGameMode.BP_MainGameMode_C|GetMultiplier _asbp_main_game_mode) (Variables|/Game/Blueprints/Gameplay/BP_MainGameMode.BP_MainGameMode_C|GetMaxMultiplier _asbp_main_game_mode)))))

(event Input|KeyboardEvents|1
  (params (Key :type Key%20Structure :default "None"))
  (:Released
    (Class|WidgetBlueprintLibrary|SetColorVisionDeficiencyType "NormalVision" 1.0 false)))

(event Input|KeyboardEvents|2
  (params (Key :type Key%20Structure :default "None"))
  (:Released
    (Class|WidgetBlueprintLibrary|SetColorVisionDeficiencyType "Deuteranope" 1.0 false)))

(event Input|KeyboardEvents|3
  (params (Key :type Key%20Structure :default "None"))
  (:Released
    (Class|WidgetBlueprintLibrary|SetColorVisionDeficiencyType "Protanope" 1.0 false)))

(event Input|KeyboardEvents|4
  (params (Key :type Key%20Structure :default "None"))
  (:Released
    (Class|WidgetBlueprintLibrary|SetColorVisionDeficiencyType "Tritanope" 1.0 false)))

(event Input|KeyboardEvents|Escape
  (params (Key :type Key%20Structure :default "None"))
  (:Pressed
    (Variables|Default|GetPlayerCharacterReference
      (:then
        (bind _pausescreenwidget (Variables|Default|GetPauseScreenWidget)
          (:then
            (Widget|RemovefromParent _pausescreenwidget)
            (Variables|Default|SetPauseScreenWidget 0))
          (:else
            (bind _returnvalue (UserInterface|CreateWidget "/Game/UI/WBP_PauseScreen.WBP_PauseScreen_C" self))
            (bind _output_get (Variables|Default|SetPauseScreenWidget _returnvalue))
            (UserInterface|Viewport|AddtoViewport _output_get 0)
            (Input|SetInputModeUIOnly self 0 "DoNotLock" false)
            (Class|Stopwatch|Stop (Variables|/Game/Blueprints/Gameplay/BP_MainGameMode.BP_MainGameMode_C|GetStopwatch (.AsBP%20Main%20Game%20Mode (Utilities|Casting|CastToBP_MainGameMode (Game|GetGameMode)))))
            (Game|SetGamePaused true))))
      (:else))))

(fn ConstructionScript)