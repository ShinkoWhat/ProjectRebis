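; BP_MainGameMode is a game mode that spawns and possesses the player's pawn once an init callback fires.
; BeginPlay binds that callback, which sets the default pawn class to BP_MainPlayer and calls PreparePawn.
; PreparePawn always spawns the pawn at the "PlayerStart" location, has player controller 0 possess it, then notifies BP_MainPlayerController through CallOnInitializePawn.
; An unconnected color vision deficiency node never runs.
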(event Custom|SpawnPlayerCallback
  (Variables|Default|SetDefaultPawnClass "/Game/Blueprints/Gameplay/BP_MainPlayer.BP_MainPlayer_C")
  (CallFunction|PreparePawn))

(event EventBeginPlay
  (EventDispatchers|BindEventtoOnInit (delegate Custom|SpawnPlayerCallback)))

(fn ConstructionScript)

(fn PreparePawn
  (bind _returnvalue (Game|GetPlayerController 0))
  (bind _returnvalue_2 (Game|SpawnActorfromClass (Variables|Default|GetDefaultPawnClass) (Math|Transform|MakeTransform (Transformation|GetActorLocation (Class|GameModeBase|FindPlayerStart (Game|GetPlayerController 0) "PlayerStart")) "0, 0, 0" "1.000000,1.000000,1.000000") "AlwaysSpawn" "MultiplyWithRoot" 0 0))
  (Pawn|Possess _returnvalue _returnvalue_2)
  (bind _asbp_main_player_controller (Utilities|Casting|CastToBP_MainPlayerController _returnvalue))
  (Default|CallOnInitializePawn _asbp_main_player_controller))