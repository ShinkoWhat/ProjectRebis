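; Player pawn Blueprint that spawns its equipped weapons at the start of play.
; BeginPlay loops over the EquippedWeapons classes, spawning each at the pawn's transform without attaching it and overwriting CurrentWeapon, so the last one spawned remains current.
; Tick prints the camera's field of view to the screen every frame as a debug readout.
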(event EventTick
  (params (DeltaSeconds :type Float%20%28single-precision%29))
  ;[1 0.0828 0.1126] Event Tick
  (Development|PrintString (Utilities|String|ToString(Float) (Variables|/Script/Engine.CameraComponent|GetFieldOfView (Variables|Default|GetCamera))) true true "(R=0.000000,G=0.660000,B=1.000000,A=1.000000)" 0.0))

(event EventBeginPlay
  ;[0.03523 0.1636 1] Begin Play
  (Utilities|FlowControl|Sequence
    (:then_0
      (for _array_element (Variables|Default|GetEquippedWeapons)
        (bind _returnvalue (Game|SpawnActorfromClass _array_element (Transformation|GetActorTransform) "Undefined" "MultiplyWithRoot" 0 0))
        (Variables|Default|SetCurrentWeapon _returnvalue)))))

(fn ConstructionScript)