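; Basic enemy character Blueprint that hurts the player on contact and awards score when killed.
; Its box overlap, gated by a DoOnce that resets on end overlap, calls the overlap handler and the player's self-hit callback.
; A death delegate updates game mode multiplier and defeat counts, feeds the scoring subsystem, spawns a Niagara explosion and destroys the actor.
; Tick copies movement velocity into the animation Blueprint.
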(event OnComponentEndOverlap(Box)
  (params (OverlappedComponent :type Primitive%20Component%20Object%20Reference) (OtherActor :type Actor%20Object%20Reference) (OtherComp :type Primitive%20Component%20Object%20Reference) (OtherBodyIndex :type Integer))
  (Utilities|FlowControl|DoOnce false) ; enters at Reset
)

(event OnComponentBeginOverlap(Box)
  (params (OverlappedComponent :type Primitive%20Component%20Object%20Reference) (OtherActor :type Actor%20Object%20Reference) (OtherComp :type Primitive%20Component%20Object%20Reference) (OtherBodyIndex :type Integer) (bFromSweep :type Boolean) (SweepResult :type Hit%20Result%20Structure%20%28by%20ref%29))
  (Utilities|FlowControl|DoOnce false
    (:Completed
      (bind _ascharacter_base (Utilities|Casting|CastToCharacterBase OtherActor))
      (if (== OtherActor _ascharacter_base)
        (Class|CharacterBase|TestOverlapHandler self 0 OtherActor 0 0 false SweepResult)
        (bind _asbp_main_player (Utilities|Casting|CastToBP_MainPlayer _ascharacter_base))
        (Default|OnSelfHitCallback _asbp_main_player)))))

(event Custom|OnDeathDelegateCallback
  (bind _asbp_main_game_mode (Utilities|Casting|CastToBP_MainGameMode (Game|GetGameMode)))
  (Default|CallOnSetMultiplier _asbp_main_game_mode)
  (Variables|/Game/Blueprints/Gameplay/BP_MainGameMode.BP_MainGameMode_C|SetTempEnemyCount _asbp_main_game_mode (+ (Variables|/Game/Blueprints/Gameplay/BP_MainGameMode.BP_MainGameMode_C|GetTempEnemyCount _asbp_main_game_mode) 1))
  (bind _structout (Utilities|Struct|SetmembersinAttemptData (Variables|/Script/ProjectRebis.BaseGamemode|GetAttemptData _asbp_main_game_mode) (+ (Utilities|Struct|BreakAttemptData (Variables|/Script/ProjectRebis.BaseGamemode|GetAttemptData _asbp_main_game_mode)) 1)))
  (Class|ScoringSubsystem|UpdateCurrentScore (Subsystems|GetScoringSubsystem) (Variables|/Game/Blueprints/Gameplay/BP_MainGameMode.BP_MainGameMode_C|GetMultiplier _asbp_main_game_mode))
  (Utilities|FlowControl|Sequence
    (:then_0
      (Niagara|SpawnSystematLocation "/Game/Assets/VFX/N_Boom.N_Boom" (Transformation|GetActorLocation))
      (Variables|Default|SetbIsAlive false))
    (:then_1
      (Development|PrintString (Utilities|String|Append "Enemies Defeated: " (Utilities|String|ToString(Integer) (Utilities|Struct|BreakAttemptData _structout)))))
    (:then_2
      (Actor|DestroyActor))))

(event EventBeginPlay
  (EventDispatchers|BindEventtoOnDeathDelegate (delegate Custom|OnDeathDelegateCallback)))

(event Collision|EventActorBeginOverlap
  (params (OtherActor :type Actor%20Object%20Reference)))

(event EventTick
  (params (DeltaSeconds :type Float%20%28single-precision%29))
  (bind _asabp_base_npc (Utilities|Casting|CastToABP_BaseNPC (Components|SkeletalMesh|GetAnimInstance (Variables|Character|GetMesh))))
  (Variables|/Game/Assets/Characters/ABP_BaseNPC.ABP_BaseNPC_C|SetVelocity _asabp_base_npc (Variables|/Script/Engine.MovementComponent|GetVelocity (Variables|Character|GetCharacterMovement))))

(fn ConstructionScript)