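; BP_BaseNPCController is the AI controller for a basic NPC, running the BT_BasicNPC behavior tree on BeginPlay.
; AI perception updates feed HandleHearing, which despite its name processes only sight stimuli from the player character.
; It sets the TargetActor blackboard key to the player while seen and clears it when sight is lost.
; LastLocation stores the stimulus location on each successful sighting update.
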(event OnTargetPerceptionUpdated(AIPerception)
  (params (Actor :type Actor%20Object%20Reference) (Stimulus :type AI%20Stimulus%20Structure))
  (CallFunction|HandleHearing Actor Stimulus))

(event EventBeginPlay
  (AI|RunBehaviorTree "/Game/Blueprints/AI/BasicEnemy/BT_BasicNPC.BT_BasicNPC"))

(event EventTick
  (params (DeltaSeconds :type Float%20%28single-precision%29)))

(fn ConstructionScript)

(fn HandleHearing
  (params (Actor :type Actor%20Object%20Reference) (Stimulus :type AI%20Stimulus%20Structure%20%28by%20ref%29))
  (bind _returnvalue (Class|AIPerceptionSystem|GetSenseClassforStimulus Stimulus))
  (if (== _returnvalue "/Script/AIModule.AISense_Sight")
    (if (== Actor (Game|GetPlayerCharacter 0))
      (AI|Components|Blackboard|SetValueasObject (Variables|Default|GetBlackboard) (Utilities|Name|MakeLiteralName "TargetActor") (Utilities|SelectObject (Game|GetPlayerCharacter 0) 0 (.bsuccessfullysensed Stimulus)))
      (if (.bsuccessfullysensed Stimulus)
        (AI|Components|Blackboard|SetValueasVector (Variables|Default|GetBlackboard) (Utilities|Name|MakeLiteralName "LastLocation") (.stimuluslocation Stimulus)))
      (else
        (return)))
    (else
      (return))))