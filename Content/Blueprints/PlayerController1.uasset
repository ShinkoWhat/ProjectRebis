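; Player controller for a cursor-aimed character that shows the mouse and adds the gameplay input mapping context.
; Light and secondary attack inputs fire event dispatchers bound to local callbacks.
; Primary attack passes the cursor hit location to the current weapon's ability instance, while the secondary callback is empty.
; Tick yaws the pawn's mesh toward the cursor hit; camera FOV logic is left unwired.
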(event Custom|PrimaryAttackCallback
  ;[0.5948 0.6891 1] Begin Play
  (CallFunction|OnMove))

(event Custom|SecondaryAttackCallback
  ;[0.5948 0.6891 1] Begin Play
)

(event Custom|OnMove
  (bind _asplayer_pawn (Utilities|Casting|CastToPlayerPawn (Variables|Default|GetPlayerPawn)))
  (bind _output_get (Variables|Default|SetCachedLocation (.location (.HitResult (Class|PlayerController|GetHitResultUnderCursorforObjects (Game|GetPlayerController 0) (Utilities|Array|MakeArray (Variables|Default|GetQueryType)) true)))))
  (Default|Primary (Variables|/Game/Blueprints/Weapons/BP_BaseWeapon.BP_BaseWeapon_C|GetAbilityInstance (Variables|/Game/Blueprints/PlayerPawn.PlayerPawn_C|GetCurrentWeapon _asplayer_pawn)) _asplayer_pawn (Math|Transform|MakeTransform _output_get "0, 0, 0" "1.000000,1.000000,1.000000")))

(event Input|EnhancedActionEvents|EnhancedInputActionIA_LightAttack
  (params (ActionValue :type Boolean) (ElapsedSeconds :type Float%20%28double-precision%29) (TriggeredSeconds :type Float%20%28double-precision%29) (InputAction :type Input%20Action%20Object%20Reference :default "/Game/Input/Actions/IA_LightAttack.IA_LightAttack"))
  ;[1 0.9042 0.2499] LightATK Input
  (:Triggered
    (Default|CallOnPrimaryAttack)))

(event Input|EnhancedActionEvents|EnhancedInputActionIA_SecondaryAttack
  (params (ActionValue :type Boolean) (ElapsedSeconds :type Float%20%28double-precision%29) (TriggeredSeconds :type Float%20%28double-precision%29) (InputAction :type Input%20Action%20Object%20Reference :default "/Game/Input/Actions/IA_SecondaryAttack.IA_SecondaryAttack"))
  ;[0.8021 0.6794 0] SecATK Input
  (:Triggered
    (Default|CallOnSecondaryAttack)))

(event EventBeginPlay
  ;[0.5948 0.6891 1] Begin Play
  (Utilities|FlowControl|Sequence
    (:then_0
      (Variables|Default|SetbShowMouseCursor true)
      (Variables|Default|SetPlayerPawn (Game|GetPlayerCharacter 0))
      (Input|AddMappingContext (PlayerController|LocalPlayerSubsystems|GetEnhancedInputLocalPlayerSubsystem (Game|GetPlayerController 0)) "/Game/Input/IMC_GameplayContext.IMC_GameplayContext" 0 "(bIgnoreAllPressedKeysUntilRelease=True,bForceImmediately=False)"))
    (:then_1
      (EventDispatchers|BindEventtoOnPrimaryAttack (delegate Custom|PrimaryAttackCallback))
      (EventDispatchers|BindEventtoOnSecondaryAttack (delegate Custom|SecondaryAttackCallback)))))

(event EventTick
  (params (DeltaSeconds :type Float%20%28single-precision%29))
  (bind _asplayer_pawn (Utilities|Casting|CastToPlayerPawn (Variables|Default|GetPlayerPawn)))
  (Transformation|SetRelativeRotation (Variables|/Game/Blueprints/PlayerPawn.PlayerPawn_C|GetSkeletalMesh _asplayer_pawn) (Math|Rotator|MakeRotator 0.0 0.0 (.yaw (Math|Rotator|FindRelativeLookatRotation (Transformation|GetRelativeTransform (Variables|/Game/Blueprints/PlayerPawn.PlayerPawn_C|GetSkeletalMesh _asplayer_pawn)) (.location (.HitResult (Class|PlayerController|GetHitResultUnderCursorforObjects (Game|GetPlayerController 0) (Utilities|Array|MakeArray (Variables|Default|GetQueryType)) true)))))) false false))

(fn ConstructionScript)