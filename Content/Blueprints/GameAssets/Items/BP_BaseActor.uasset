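; BP_BaseActor is a destructible item actor that loses HP when the player pawn hits its static mesh.
; Each hit subtracts the damage value of the pawn's current weapon, and other actors deal none.
; Tick polls HP and fires the OnDestroy dispatcher at zero or below.
; The bound callback calls OnSetTimeDilation on NewGameMode, then destroys the actor.
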(event OnComponentHit(StaticMesh)
  (params (HitComponent :type Primitive%20Component%20Object%20Reference) (OtherActor :type Actor%20Object%20Reference) (OtherComp :type Primitive%20Component%20Object%20Reference) (NormalImpulse :type Vector :default "0, 0, 0") (Hit :type Hit%20Result%20Structure%20%28by%20ref%29))
  (CallFunction|ReduceHp OtherActor))

(event Custom|OnDestroyCallback
  (bind _asnew_game_mode (Utilities|Casting|CastToNewGameMode (Game|GetGameMode)))
  (Default|CallOnSetTimeDilation _asnew_game_mode)
  (Actor|DestroyActor))

(event EventBeginPlay
  (EventDispatchers|BindEventtoOnDestroy (delegate Custom|OnDestroyCallback)))

(event EventTick
  (params (DeltaSeconds :type Float%20%28single-precision%29))
  (Utilities|FlowControl|Sequence
    (:then_0
      (if (<= (Variables|Default|GetHP) 0.0)
        (Default|CallOnDestroy)))))

(fn ConstructionScript)

(fn ReduceHp
  (params (Object :type Object%20Object%20Reference))
  (bind _asplayer_pawn (Utilities|Casting|CastToPlayerPawn Object))
  (Variables|Default|SetHP (- (Variables|Default|GetHP) (.damage (Variables|/Game/Blueprints/Weapons/BP_BaseWeapon.BP_BaseWeapon_C|GetWeaponInfo (Variables|/Game/Blueprints/PlayerPawn.PlayerPawn_C|GetCurrentWeapon _asplayer_pawn))))))