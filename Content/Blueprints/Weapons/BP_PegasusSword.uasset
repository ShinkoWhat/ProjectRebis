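; Pegasus sword weapon whose primary ability dashes the player horizontally toward a target location via LaunchCharacter.
; Each attack raises a counter that accelerates dash velocity up to a cap, further scaled by the game mode's log Multiplier, until a reset callback restores defaults.
; Mesh overlaps with NPCBase actors go to the player's TestOverlapHandler, gated by a DoOnce that resets on end overlap.
; Secondary and transition abilities are print-string placeholders.
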(event OnComponentEndOverlap(SkeletalMeshComponent)
  (params (OverlappedComponent :type Primitive%20Component%20Object%20Reference) (OtherActor :type Actor%20Object%20Reference) (OtherComp :type Primitive%20Component%20Object%20Reference) (OtherBodyIndex :type Integer))
  (Utilities|FlowControl|DoOnce false) ; enters at Reset
)

(event OnComponentBeginOverlap(SkeletalMeshComponent)
  (params (OverlappedComponent :type Primitive%20Component%20Object%20Reference) (OtherActor :type Actor%20Object%20Reference) (OtherComp :type Primitive%20Component%20Object%20Reference) (OtherBodyIndex :type Integer) (bFromSweep :type Boolean) (SweepResult :type Hit%20Result%20Structure%20%28by%20ref%29))
  (Utilities|FlowControl|DoOnce false
    (:Completed
      (bind _ascharacter_base (Utilities|Casting|CastToCharacterBase (Game|GetPlayerCharacter 0)))
      (if (Utilities|ClassIsChildOf (Utilities|GetClass OtherActor) "/Script/ProjectRebis.NPCBase")
        (Class|CharacterBase|TestOverlapHandler _ascharacter_base 0 OtherActor 0 0 false SweepResult)))))

(event Custom|OnResetAtkCountCallback
  (Variables|Default|SetAtkCount 0)
  (Variables|Default|SetCurrentVelocity 1.5e+03))

(event EventBeginPlay
  (EventDispatchers|BindEventtoResetAtkCount (delegate Custom|OnResetAtkCountCallback)))

(event Collision|EventActorBeginOverlap
  (params (OtherActor :type Actor%20Object%20Reference)))

(event EventTick
  (params (DeltaSeconds :type Float%20%28single-precision%29)))

(event EventTransitionAbility
  (params (PlayerReference :type Character%20Base%20Object%20Reference) (TargetLocation :type Vector :default "0, 0, 0"))
  (Development|PrintString "Hello"))

(event EventSecondaryAbility
  (params (PlayerReference :type Character%20Base%20Object%20Reference) (TargetLocation :type Vector :default "0, 0, 0"))
  (Development|PrintString "Hello"))

(event EventPrimaryAbility
  (params (PlayerReference :type Character%20Base%20Object%20Reference) (TargetLocation :type Vector :default "0, 0, 0") (MinVelocity :type Float%20%28double-precision%29) (MaxVelocity :type Float%20%28double-precision%29))
  (bind (_x _y _z) (Math|Vector|BreakVector TargetLocation))
  (CallFunction|AtkCounter)
  (bind _asbp_main_player (Utilities|Casting|CastToBP_MainPlayer PlayerReference))
  (bind _asbp_main_game_mode (Utilities|Casting|CastToBP_MainGameMode (Game|GetGameMode)))
  (bind _velocity (CallFunction|Accelerate (Math|Float|Lerp 0.0 (Variables|Default|GetWeaponAcceleration) (/ (Variables|Default|GetAtkCount) (Variables|Default|GetMaxAtkCount)))))
  (bind _output_get (Variables|Default|SetCurrentVelocity _velocity))
  (Character|LaunchCharacter _asbp_main_player (* (Math|Vector|ProjectVectorontoPlane (Math|Vector|GetUnitDirection(Vector) (Math|Vector|MakeVector (.x (Transformation|GetActorLocation _asbp_main_player)) (.y (Transformation|GetActorLocation _asbp_main_player)) (.z (Transformation|GetActorLocation _asbp_main_player))) (Math|Vector|MakeVector _x _y _z)) "0.000000,0.000000,1.000000") _output_get (Math|Float|Lerp 1.0 1.8 (/ (Math|Float|Loge (Variables|/Game/Blueprints/Gameplay/BP_MainGameMode.BP_MainGameMode_C|GetMultiplier _asbp_main_game_mode)) (Variables|/Game/Blueprints/Gameplay/BP_MainGameMode.BP_MainGameMode_C|GetMaxMultiplier _asbp_main_game_mode)))) false false))

(fn ConstructionScript)

(fn Accelerate
  (params (DeltaVelocity :type Float%20%28double-precision%29))
  (bind _weaponmaxvelocity (Variables|Default|GetWeaponMaxVelocity))
  (bind _currentvelocity (Variables|Default|GetCurrentVelocity))
  (bind _returnvalue (+ _currentvelocity DeltaVelocity))
  (if (<= _returnvalue _weaponmaxvelocity)
    (return _returnvalue)
    (else
      (return _weaponmaxvelocity))))

(fn AtkCounter
  (if (<= (Variables|Default|GetAtkCount) (Variables|Default|GetMaxAtkCount))
    (Variables|Default|SetAtkCount (+ (Variables|Default|GetAtkCount) 1))
    (else
      (Variables|Default|SetAtkCount (Variables|Default|GetMaxAtkCount)))))