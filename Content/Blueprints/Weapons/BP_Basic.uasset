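; BP_Basic is a basic weapon Blueprint, apparently a test weapon, that sets up its ability and weapon info when play begins.
; After calling the parent BeginPlay, it assigns BP_Movement as its Ability class.
; If no valid AbilityInstance exists, it constructs one from that class and fills WeaponInfo with hardcoded test data in the same branch.
; Overlap and Tick events are disabled, and the construction script only calls the parent.
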(event EventBeginPlay
  (|CallParentFunction)
  (Variables|Default|SetAbility "/Game/Blueprints/Weapons/Abilities/BP_Movement.BP_Movement_C")
  (Variables|Default|GetAbilityInstance
    (:then)
    (:else
      (bind _returnvalue (Game|ConstructObjectfromClass (Variables|Default|GetAbility)))
      (Variables|Default|SetAbilityInstance _returnvalue)
      (Variables|Default|SetWeaponInfo (Utilities|Struct|MakeS_WeaponInfo "TestWeapon" "TEST" "NewEnumerator0" 1e+02 4e+03)))))

(event Collision|EventActorBeginOverlap
  (params (OtherActor :type Actor%20Object%20Reference))
  (|CallParentFunction OtherActor) ; This node is disabled and will not be called.\nDrag off pins to build functionality.
)

(event EventTick
  (params (DeltaSeconds :type Float%20%28single-precision%29))
  (|CallParentFunction DeltaSeconds) ; This node is disabled and will not be called.\nDrag off pins to build functionality.
)

(fn ConstructionScript
  (|CallParentFunction))