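; BP_Movement is a weapon ability that moves the player pawn by launching it relative to a target destination.
; Primary launches toward the destination, rotating the direction by the destination's pitch and scaling it by the current weapon's WeaponSpeed.
; Secondary launches horizontally away from the destination at a reduced fraction of that speed.
; Both call their parent version first and add to existing velocity rather than overriding it.
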(fn Primary
  (params (PawnReference :type Character%20Object%20Reference) (LocationDestination :type Transform))
  (bind (_location _rotation) (Math|Transform|BreakTransform LocationDestination))
  (|CallParentFunction 0 "")
  (bind _asplayer_pawn (Utilities|Casting|CastToPlayerPawn PawnReference))
  (Character|LaunchCharacter PawnReference (* (Math|Vector|RotateVector (Math|Vector|GetUnitDirection(Vector) (Transformation|GetActorLocation PawnReference) (Math|Vector|MakeVector (.x _location) (.y _location) (.z _location))) (Math|Rotator|MakeRotator 0.0 (.pitch _rotation) 0.0)) (.weaponspeed (Variables|/Game/Blueprints/Weapons/BP_BaseWeapon.BP_BaseWeapon_C|GetWeaponInfo (Variables|/Game/Blueprints/PlayerPawn.PlayerPawn_C|GetCurrentWeapon _asplayer_pawn)))) false false))

(fn Secondary
  (params (PawnReference :type Character%20Object%20Reference) (LocationDestination :type Transform))
  (bind _location (Math|Transform|BreakTransform LocationDestination))
  (bind _returnvalue (Transformation|GetActorLocation PawnReference))
  (|CallParentFunction 0 "")
  (bind _asplayer_pawn (Utilities|Casting|CastToPlayerPawn PawnReference))
  (Character|LaunchCharacter PawnReference (* (* (Math|Vector|GetUnitDirection(Vector) (Math|Vector|MakeVector (.x _returnvalue) (.y _returnvalue) (.z _returnvalue)) (Math|Vector|MakeVector (.x _location) (.y _location) (.z _returnvalue))) -1) (.weaponspeed (Variables|/Game/Blueprints/Weapons/BP_BaseWeapon.BP_BaseWeapon_C|GetWeaponInfo (Variables|/Game/Blueprints/PlayerPawn.PlayerPawn_C|GetCurrentWeapon _asplayer_pawn))) 0.4) false false))