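; Game mode that runs a slow-motion effect, started and cancelled through bound time-dilation events.
; A timeline drives global time dilation and the player camera's FOV, while flagging time as slowed and setting the controller's movement state.
; Cancel stops and repositions the timeline and clears the flag; the movement-state reset after finishing is left unconnected.
; Tick prints the current dilation as debug output.
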(event Custom|OnTimeDilate
  (bind (_direction _timedilation _fov) (Timeline|TimeDilation Play)
    (:Update
      (Utilities|Time|SetGlobalTimeDilation (Math|Float|Lerp 0.2 1.0 _timedilation))
      (Camera|SetFieldOfView (Variables|/Game/Blueprints/PlayerPawn.PlayerPawn_C|GetCamera (Variables|Default|GetPlayer)) (Math|Float|Lerp 1e+02 1.1e+02 _fov))
      (Variables|Default|SetIsTimeSlowed true)
      (bind _asplayer_controller_1 (Utilities|Casting|CastToPlayerController1 (Game|GetPlayerController 0)))
      (Variables|/Game/Blueprints/PlayerController1.PlayerController1_C|SetMovementState _asplayer_controller_1 "NewEnumerator1"))
    (:Finished
      (Variables|Default|SetIsTimeSlowed false)
      (bind _asplayer_controller_1_2 (Utilities|Casting|CastToPlayerController1 (Game|GetPlayerController 0))))))

(event Custom|TimeDilationCancel
  (Variables|Default|SetIsTimeSlowed false)
  (Utilities|FlowControl|Sequence
    (:then_0
      (bind (_direction _timedilation _fov) (Timeline|TimeDilation Stop)
        (:Update
          (Utilities|Time|SetGlobalTimeDilation (Math|Float|Lerp 0.2 1.0 _timedilation))
          (Camera|SetFieldOfView (Variables|/Game/Blueprints/PlayerPawn.PlayerPawn_C|GetCamera (Variables|Default|GetPlayer)) (Math|Float|Lerp 1e+02 1.1e+02 _fov))
          (Variables|Default|SetIsTimeSlowed true)
          (bind _asplayer_controller_1 (Utilities|Casting|CastToPlayerController1 (Game|GetPlayerController 0)))
          (Variables|/Game/Blueprints/PlayerController1.PlayerController1_C|SetMovementState _asplayer_controller_1 "NewEnumerator1"))
        (:Finished
          (Variables|Default|SetIsTimeSlowed false)
          (bind _asplayer_controller_1_2 (Utilities|Casting|CastToPlayerController1 (Game|GetPlayerController 0))))))
    (:then_1
      (Timeline|TimeDilation SetNewTime))))

(event EventBeginPlay
  (EventDispatchers|BindEventtoOnSetTimeDilation (delegate Custom|OnTimeDilate))
  (EventDispatchers|BindEventtoOnTimeDilationCancel (delegate Custom|TimeDilationCancel))
  (bind _asplayer_pawn (Utilities|Casting|CastToPlayerPawn (Game|GetPlayerCharacter 0)))
  (Variables|Default|SetPlayer _asplayer_pawn))

(event EventTick
  (params (DeltaSeconds :type Float%20%28single-precision%29))
  (Development|PrintString (Utilities|String|ToString(Float) (Class|GameplayStatics|GetGlobalTimeDilation)) true true "(R=1.000000,G=0.000000,B=0.911979,A=1.000000)" 0.0))

(fn ConstructionScript)