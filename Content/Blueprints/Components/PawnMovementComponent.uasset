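; Pawn movement component that drives a physics-simulated capsule root from the owning pawn's movement input.
; BeginPlay configures capsule physics and starts a looping fixed-step timer, while Tick caches normalized input and zeroes capsule rotation to keep it upright.
; Each fixed step accelerates velocity toward input times max speed, damping motion on the plane perpendicular to gravity, then writes it back.
; Engine gravity is enabled; the custom gravity function is called disabled.
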(event Custom|FixedTick
  (Variables|Default|SetVelocity (Transformation|GetComponentVelocity (Variables|Default|GetCapsule%20Collision)))
  (CallFunction|ApplyGravity false)
  (CallFunction|MovementVelocity (Variables|Default|GetMax%20Speed) (Variables|Default|GetAcceleration))
  (Class|PrimitiveComponent|SetAllPhysicsLinearVelocity (Variables|Default|GetCapsule%20Collision) (Variables|Default|GetVelocity) false))

(event EventBeginPlay
  (bind _aspawn (Utilities|Casting|CastToPawn (Components|GetOwner)))
  (bind _output_get (Variables|Default|SetParent%20Pawn _aspawn))
  (bind _ascapsule_collision (Utilities|Casting|CastToCapsuleComponent (Variables|/Script/Engine.Actor|GetRootComponent _output_get)))
  (Variables|Default|SetCapsule%20Collision _ascapsule_collision)
  (CallFunction|ConfigurePhysics)
  (bind _output_get_2 (Variables|Default|SetDeltaTime (/ (Math|Float|MakeLiteralFloat 1.0) (Math|Float|MakeLiteralFloat 2.5e+02))))
  (Utilities|Time|SetTimerbyEvent (delegate Custom|FixedTick) _output_get_2 true))

(event EventTick
  (params (DeltaSeconds :type Float%20%28single-precision%29))
  (bind _parent_pawn (Variables|Default|GetParent%20Pawn)
    (:then
      (bind _returnvalue (Class|Pawn|ConsumeMovementInputVector _parent_pawn))
      (Variables|Default|SetInput (Math|Vector|Normalize _returnvalue))
      (Transformation|SetWorldRotation (Variables|Default|GetCapsule%20Collision) "0, 0, 0" false false))
    (:else)))

(fn ConfigurePhysics
  (Components|Tick|SetTickGroup "TG_PostPhysics")
  (Physics|SetSimulatePhysics (Variables|Default|GetCapsule%20Collision) true)
  (Physics|SetEnableGravity (Variables|Default|GetCapsule%20Collision) true)
  (Collision|SetCollisionProfileName (Variables|Default|GetCapsule%20Collision) "Pawn" true :!class /Script/Engine.PrimitiveComponent)
  (Class|PrimitiveComponent|SetPhysMaterialOverride (Variables|Default|GetCapsule%20Collision) "/Game/Blueprints/Assets/PawnPhysicalMaterial.PawnPhysicalMaterial"))

(fn ApplyGravity
  (params (IsEnabled :type Boolean))
  (if IsEnabled
    (Variables|Default|SetVelocity (+ (Variables|Default|GetVelocity) (* (* (Variables|Default|GetGravityDirection) (Math|Float|MakeLiteralFloat 9.8e+02)) (Variables|Default|GetDeltaTime))))))

(fn MovementVelocity
  (params (MaxSpeed :type Float%20%28double-precision%29) (Acceleration :type Float%20%28double-precision%29))
  (Variables|Default|SetVelocity (+ (* (- (* (* (Variables|Default|GetInput) MaxSpeed) Acceleration) (* (Math|Vector|ProjectVectorontoPlane (Variables|Default|GetVelocity) (Variables|Default|GetGravityDirection)) Acceleration)) (Variables|Default|GetDeltaTime)) (Variables|Default|GetVelocity))))