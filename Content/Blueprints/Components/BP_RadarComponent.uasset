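; Radar component meant to show up to four enemies on a material-driven plane belonging to BP_MainPlayer.
; VecUpdate writes each enemy's offset from the player into the vector parameters EnemyVec1 to EnemyVec4 on that plane's materials.
; BeginPlay casts the owner but sets the player reference to None.
; Tick is empty and the VecUpdate call is disconnected, so the radar never updates from this graph.
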(event EventBeginPlay
  (Utilities|Casting|CastToBP_MainPlayer (Components|GetOwner))
  (Variables|Default|SetPlayerCharacterReference 0))

(event EventTick
  (params (DeltaSeconds :type Float%20%28single-precision%29)))

(fn VecUpdate
  (params (ActorArray :type Array%20of%20Actor%20Object%20References))
  (bind _playercharacterreference (Variables|Default|GetPlayerCharacterReference))
  (bind _returnvalue (Transformation|GetActorLocation _playercharacterreference))
  (bind _plane (Variables|/Game/Blueprints/Gameplay/BP_MainPlayer.BP_MainPlayer_C|GetPlane _playercharacterreference))
  (Utilities|FlowControl|Sequence
    (:then_0
      (Rendering|Material|SetVectorParameterValueonMaterials _plane "EnemyVec1" (- (Transformation|GetActorLocation (Utilities|Array|Get(acopy) ActorArray)) _returnvalue)))
    (:then_1
      (Rendering|Material|SetVectorParameterValueonMaterials _plane "EnemyVec2" (- (Transformation|GetActorLocation (Utilities|Array|Get(acopy) ActorArray 1)) _returnvalue)))
    (:then_2
      (Rendering|Material|SetVectorParameterValueonMaterials _plane "EnemyVec3" (- (Transformation|GetActorLocation (Utilities|Array|Get(acopy) ActorArray 2)) _returnvalue)))
    (:then_3
      (Rendering|Material|SetVectorParameterValueonMaterials _plane "EnemyVec4" (- (Transformation|GetActorLocation (Utilities|Array|Get(acopy) ActorArray 3)) _returnvalue)))))